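; BP_Accounting is a LVL3 trigger box actor that tallies fallen Jenga blocks and detects the win.
; After a short startup delay, it caches the level widget, player and game mode.
; Each overlapping block is destroyed: gold targets update the score and the player's remaining count, while others deduct time.
; When no gold blocks remain, it clears the player's timer and shows the victory widget with UI-only input.
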(event `self.ReceiveBeginPlay`
  ; Récupération du widget du level, du player et du game mode
  (`KismetSystemLibrary.Delay` 2.0)
  (bind _foundwidgets (`WidgetBlueprintLibrary.GetAllWidgetsOfClass` "/Game/_Game/WBP/WBP_LVL3.WBP_LVL3_C"))
  (set `self.WBP LVL3` (`|GetArrayItem` _foundwidgets))
  (bind _asbp_player (cast `/Game/_Game/Blueprints/LVL3/BP_Player` (`GameplayStatics.GetPlayerCharacter` 0)))
  (set `self.As BP Player` _asbp_player)
  (bind _asgm_default_lvl3 (cast `/Game/_Game/Blueprints/LVL3/GM_Default_LVL3` (`GameplayStatics.GetGameMode`)))
  (set `self.As GM Default LVL3` _asgm_default_lvl3))

(event `self.Box.OnComponentBeginOverlap`
  (params (OverlappedComponent :type "PrimitiveComponent Object Reference") (OtherActor :type "Actor Object Reference") (OtherComp :type "PrimitiveComponent Object Reference") (OtherBodyIndex :type Integer) (bFromSweep :type Boolean) (SweepResult :type "HitResult Structure (by ref)"))
  (bind _returnvalue (`GameplayStatics.GetPlayerController` 0))
  (bind _as_bp_player (`self.As BP Player`))
  ; Update du temps ou du score en fonction du jenga qui est tombé
  (bind _asbp_jenga_block (cast `/Game/_Game/Blueprints/LVL3/BP_JengaBlock` OtherActor))
  (if (`/Game/_Game/Blueprints/LVL3/BP_JengaBlock.IsTarget?` _asbp_jenga_block)
    (`self.K2_DestroyActor` OtherActor)
    (bind _result (`/Engine/EditorBlueprintResources/StandardMacros.IncrementInt` (`self.ActualScore`))
      (:`  `
        (`/Game/_Game/WBP/WBP_LVL3.UpdateScore` (`self.WBP LVL3`) _result)
        (bind _result_2 (`/Engine/EditorBlueprintResources/StandardMacros.DecrementInt` (`/Game/_Game/Blueprints/LVL3/BP_Player.GoldJengaRemaining` (`self.As BP Player`)))
          (:`  `
            ; Si il reste plus de jenga doré, affiche le widget de victoire
            (if (== _result_2 0)
              (`KismetSystemLibrary.K2_ClearAndInvalidateTimerHandle` (`/Game/_Game/Blueprints/LVL3/BP_Player.TimerByEvent` (`self.As BP Player`)))
              (bind _returnvalue_2 (`|CreateWidget` "/Game/_Game/WBP/WBP_Victory.WBP_Victory_C"))
              (`UserWidget.AddToViewport` _returnvalue_2 0)
              (set `PlayerController.bShowMouseCursor` true _returnvalue)
              (`WidgetBlueprintLibrary.SetInputMode_UIOnlyEx` _returnvalue null))))))
    (else
      (`self.K2_DestroyActor` OtherActor)
      (set `/Game/_Game/Blueprints/LVL3/BP_Player.TimeRemaining` (- (`/Game/_Game/Blueprints/LVL3/BP_Player.TimeRemaining` _as_bp_player) 2.0) _as_bp_player))))

(fn `UserConstructionScript`)