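; BP_Wind is a wind zone that pushes the jetpack player while they are inside it.
; On BeginPlay it caches the player pawn and starts a timeline whose curve modulates the wind, apparently switching it on and off.
; Each timeline update adds force to the player's Sphere along the Arrow's forward vector, scaled by WindStrength.
; WindZone overlaps set the inside flag without checking which actor triggered them.
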(event `self.ReceiveBeginPlay`
  (bind _asbp_jetpack_player (cast `/Game/_Game/Blueprints/LVL1/BP_JetpackPlayer` (`GameplayStatics.GetPlayerPawn` 0)))
  (set `self.As BP Jetpack Player` _asbp_jetpack_player)
  (bind (_direction _turn_on___off) (`Timeline|Turn Wind ON/OFF`)
    (:`Update`
      (if (`self.IsPlayerInside?`)
        (`PrimitiveComponent.AddForce` (`/Game/_Game/Blueprints/LVL1/BP_JetpackPlayer.Sphere` (`self.As BP Jetpack Player`)) (* (* _turn_on___off (`self.WindStrength`)) (`SceneComponent.GetForwardVector` (`self.Arrow`))) "None" false)))))

(event `self.WindZone.OnComponentBeginOverlap`
  (params (OverlappedComponent :type "PrimitiveComponent Object Reference") (OtherActor :type "Actor Object Reference") (OtherComp :type "PrimitiveComponent Object Reference") (OtherBodyIndex :type Integer) (bFromSweep :type Boolean) (SweepResult :type "HitResult Structure (by ref)"))
  (set `self.IsPlayerInside?` true))

(event `self.WindZone.OnComponentEndOverlap`
  (params (OverlappedComponent :type "PrimitiveComponent Object Reference") (OtherActor :type "Actor Object Reference") (OtherComp :type "PrimitiveComponent Object Reference") (OtherBodyIndex :type Integer))
  (set `self.IsPlayerInside?` false))

(fn `UserConstructionScript`)