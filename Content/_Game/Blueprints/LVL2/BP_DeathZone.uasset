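; BP_DeathZone is a kill volume in LVL2 that respawns the sphere when it falls in.
; On BeginPlay it finds and caches the BP_PlatformPlayer in the level.
; When a BP_Sphere overlaps the DeathZone component, it destroys that sphere and, after a short delay, spawns a new one at the platform's SpawnPoint transform.
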(event `self.ReceiveBeginPlay`
  ; Récupération de la plateforme
  (bind _returnvalue (`GameplayStatics.GetActorOfClass` "/Game/_Game/Blueprints/LVL2/BP_PlatformPlayer.BP_PlatformPlayer_C"))
  (`/Engine/EditorBlueprintResources/StandardMacros.IsValid` _returnvalue
    (:`Is Valid`
      (set `self.As BP_PlatformPlayer` _returnvalue))))

(event `self.DeathZone.OnComponentBeginOverlap`
  (params (OverlappedComponent :type "PrimitiveComponent Object Reference") (OtherActor :type "Actor Object Reference") (OtherComp :type "PrimitiveComponent Object Reference") (OtherBodyIndex :type Integer) (bFromSweep :type Boolean) (SweepResult :type "HitResult Structure (by ref)"))
  ; Spawn d'une nouvelle sphère lorsque l'ancienne tombe dans la death zone
  (cast `/Game/_Game/Blueprints/LVL2/BP_Sphere` OtherActor)
  (`self.K2_DestroyActor` OtherActor)
  (`KismetSystemLibrary.Delay` 0.5)
  (`|SpawnActorFromClass` "/Game/_Game/Blueprints/LVL2/BP_Sphere.BP_Sphere_C" (`SceneComponent.K2_GetComponentToWorld` (`/Game/_Game/Blueprints/LVL2/BP_PlatformPlayer.SpawnPoint` (`self.As BP_PlatformPlayer`))) "Undefined" "MultiplyWithRoot" null null))

(fn `UserConstructionScript`)