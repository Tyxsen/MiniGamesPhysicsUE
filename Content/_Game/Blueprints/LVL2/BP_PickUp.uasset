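; BP_PickUp is an LVL2 pickup that opens the red wall when a BP_Sphere overlaps its cube.
; BeginPlay finds BP_PlatformPlayer and caches the relative start position of its WallToOpen reference, plus an end position below it.
; On overlap, the OpeningDoor timeline lerps the wall downward, while a DoOnce on its update destroys the pickup's cube component.
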(event `self.ReceiveBeginPlay`
  ; Set les positions que le mur rouge devra avoir si le pick up est récupéré
  (bind _returnvalue (`GameplayStatics.GetActorOfClass` "/Game/_Game/Blueprints/LVL2/BP_PlatformPlayer.BP_PlatformPlayer_C"))
  (`/Engine/EditorBlueprintResources/StandardMacros.IsValid` _returnvalue
    (:`Is Valid`
      (bind _output_get (set `self.As BP PlatformPlayer` _returnvalue))
      (bind _output_get_2 (set `self.PosStart` (`SceneComponent.RelativeLocation` (`/Game/_Game/Blueprints/LVL2/BP_PlatformPlayer.WallToOpen` _output_get))))
      (set `self.PosEnd` (+ _output_get_2 (0.0 0.0 -100.0))))))

(event `self.Cube.OnComponentBeginOverlap`
  (params (OverlappedComponent :type "PrimitiveComponent Object Reference") (OtherActor :type "Actor Object Reference") (OtherComp :type "PrimitiveComponent Object Reference") (OtherBodyIndex :type Integer) (bFromSweep :type Boolean) (SweepResult :type "HitResult Structure (by ref)"))
  ; Timeline pour déplacer le mur rouge lorsque le pick up est récupéré + destroy du pick up
  (bind _asbp_sphere (cast `/Game/_Game/Blueprints/LVL2/BP_Sphere` OtherActor))
  (`/Engine/EditorBlueprintResources/StandardMacros.IsValid` _asbp_sphere
    (:`Is Valid`
      (`KismetSystemLibrary.PrintString` "L'objet a été récupéré, ouverture de la porte !" true true (struct :`G` 1.0 :`A` 1.0) 5.0)
      (bind (_direction _alpha) (`Timeline|OpeningDoor` :!via `PlayFromStart`)
        (:`Update`
          (`SceneComponent.K2_SetRelativeLocation` (`/Game/_Game/Blueprints/LVL2/BP_PlatformPlayer.WallToOpen` (`self.As BP PlatformPlayer`)) (`KismetMathLibrary.VLerp` (`self.PosStart`) (`self.PosEnd`) _alpha) false false)
          (`/Engine/EditorBlueprintResources/StandardMacros.DoOnce` false
            (:`Completed`
              (`ActorComponent.K2_DestroyComponent` (`self.Cube`)))))))))

(fn `UserConstructionScript`)